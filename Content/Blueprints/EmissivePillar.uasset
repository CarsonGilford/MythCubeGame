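; EmissivePillar is an actor made of fifteen cubes that light up one after another by switching to the TRed material.
; BeginPlay gathers the cubes into an array and reverses it, so the sequence runs from Cube14 to Cube0.
; LightUpTheCubes, which nothing in this graph calls, starts a looping timer that changes one cube per tick of the timer and clears itself after the last.
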(event `self.ReceiveBeginPlay`
  (bind _output_get (set `self.Cubes` (`|MakeArray` (`self.Cube0`) (`self.Cube1`) (`self.Cube2`) (`self.Cube3`) (`self.Cube4`) (`self.Cube5`) (`self.Cube6`) (`self.Cube7`) (`self.Cube8`) (`self.Cube9`) (`self.Cube10`) (`self.Cube11`) (`self.Cube12`) (`self.Cube13`) (`self.Cube14`))))
  (`KismetArrayLibrary.Array_Reverse` _output_get))

(event `LightUpTheCubes`
  (bind _returnvalue (`KismetSystemLibrary.K2_SetTimerDelegate` (delegate `LightUpACube`) (`self.Time`) true))
  (set `self.TimerHandle` _returnvalue))

(event `LightUpACube`
  (bind _counter (`self.counter`))
  (`PrimitiveComponent.SetMaterial` (`|GetArrayItem` (`self.Cubes`) _counter) 0 "/Game/Geometry/Meshes/textures/TRed.TRed")
  (`/Engine/EditorBlueprintResources/StandardMacros.IncrementInt` _counter
    (:`  `
      (if (not (< (`self.counter`) (`KismetArrayLibrary.Array_Length` (`self.Cubes`))))
        (`KismetSystemLibrary.K2_ClearAndInvalidateTimerHandle` (`self.TimerHandle`))))))

(fn `UserConstructionScript`)