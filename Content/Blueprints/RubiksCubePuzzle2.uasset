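; Interactive 2x2x2 Rubik's cube puzzle actor in which three dog heads and a stub must share one side.
; Clicking a side's collision box highlights its overlapping blocks, which input re-parents to a pivot for timeline quarter turns.
; Dog heads rotate on click, and the whole cube can be dragged or flipped.
; Tick detects the solve via box overlaps, then locks turning, snaps the cube upright and aligns the heads.
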(event `self.ReceiveTick`
  (params (DeltaSeconds :type "Float (single-precision)"))
  (bind (_returnvalue_x _returnvalue_y _returnvalue_z) (`KismetMathLibrary.BreakVector` (`self.K2_GetActorLocation`)))
  (bind _dog_head_3 (`self.dog head 3`))
  (bind _dog_head_2 (`self.dog head 2`))
  (bind _dog_head_1 (`self.dog head 1`))
  (bind _boxcontainspieces (`self.BoxContainsPieces`))
  (bind (_returnvalue_roll _returnvalue_pitch) (`KismetMathLibrary.BreakRotator` (`SceneComponent.K2_GetComponentRotation` _boxcontainspieces)))
  (bind _roll (.roll (`self.RubiksCubeCurrentRotation`)))
  (bind (_returnvalue_x_2 _returnvalue_y_2 _returnvalue_z_2) (`KismetMathLibrary.BreakVector` (`SceneComponent.K2_GetComponentLocation` (`self.BoxContainsPieces`))))
  (bind _returnvalue (`SceneComponent.K2_GetComponentLocation` (`self.BoxContainsPieces`)))
  (bind (_returnvalue_x_3 _returnvalue_y_3 _returnvalue_z_3) (`KismetMathLibrary.BreakVector` (`SceneComponent.K2_GetComponentLocation` _boxcontainspieces)))
  (bind (_returnvalue_roll_2 _returnvalue_pitch_2 _returnvalue_yaw) (`KismetMathLibrary.BreakRotator` (`KismetMathLibrary.ComposeRotators` (`KismetMathLibrary.FindLookAtRotation` _returnvalue (`self.K2_GetActorLocation`)) (`KismetMathLibrary.FindLookAtRotation` _returnvalue (`KismetMathLibrary.MakeVector` _returnvalue_x_2 _returnvalue_y_2 (+ _returnvalue_z_2 1000.0))))))
  ;[1 1 1] cube highlighting
  (`|ExecutionSequence`
    (:`then_0`
      (if (and (!= (`.HitComponent` (`GameplayStatics.BreakHitResult` (`PlayerController.GetHitResultUnderCursorByChannel` (`GameplayStatics.GetPlayerController` 0) "TraceTypeQuery1" true))) (`self.SelectedCollisionBox`)) (`self.CanTurn?`))
        (for _array_element (`self.Overlapping Blocks`)
          (`self.UnHighlightCube` (struct) _array_element))
        (`KismetArrayLibrary.Array_Clear` (`self.Overlapping Blocks`))
        (set `self.SelectedCollisionBox` null)))
    (:`then_1`
      ;[1 1 1] check if puzzle 2 is solved
      (if (`self.puzzle1Solved`)
        ;[1 1 1] puzzle 1 solved!
        (`/Engine/EditorBlueprintResources/StandardMacros.DoOnce` false
          (:`Completed`
            (set `self.CanTurn?` false)
            (set `self.RubiksCubeCurrentRotation` (`self.K2_GetActorRotation`))
            (set `self.LookAtRot` (`KismetMathLibrary.MakeRotator` (* (`KismetMathLibrary.Round` (/ _returnvalue_roll_2 90.0)) 90.0) (* (`KismetMathLibrary.Round` (/ _returnvalue_pitch_2 90.0)) 90.0) (* (`KismetMathLibrary.Round` (/ _returnvalue_yaw 90.0)) 90.0)))
            (bind (_direction _lerp) (`Timeline|Timeline_0` :!via `PlayFromStart`)
              (:`Update`
                (`self.K2_SetActorRotation` (`KismetMathLibrary.RLerp` (`self.RubiksCubeCurrentRotation`) (`self.LookAtRot`) _lerp)))
              (:`Finished`
                (if (and (< _returnvalue_z_3 _returnvalue_z) (`KismetMathLibrary.NearlyEqual_FloatFloat` _returnvalue_roll 0.0 5.0) (`KismetMathLibrary.NearlyEqual_FloatFloat` _returnvalue_pitch 0.0 5.0))
                  (set `self.Direction` 1.0)
                  (set `self.RubiksCubeCurrentRotation` (`self.K2_GetActorRotation`))
                  (bind (_direction_2 _lerp_2) (`Timeline|Timeline_2` :!via `PlayFromStart`)
                    (:`Update`
                      (set `self.CanTurn?` false)
                      (`self.K2_SetActorRotation` (`KismetMathLibrary.MakeRotator` (`KismetMathLibrary.Lerp` _roll (+ _roll (* (`self.Direction`) 180.0)) _lerp_2) (.pitch (`self.RubiksCubeCurrentRotation`)) (.yaw (`self.RubiksCubeCurrentRotation`)))))
                    (:`Finished`
                      (set `self.CanTurn?` false)
                      (bind (_direction_3 _lerp_3) (`Timeline|Timeline_1` :!via `PlayFromStart` :!label _label)
                        (:`Update`
                          (`SceneComponent.K2_SetRelativeRotation` _dog_head_3 (`KismetMathLibrary.RLerp` (`SceneComponent.RelativeRotation` _dog_head_3) (struct :`Yaw` -90.0) _lerp_3 true) false false)
                          (`SceneComponent.K2_SetRelativeRotation` _dog_head_2 (`KismetMathLibrary.RLerp` (`SceneComponent.RelativeRotation` _dog_head_2) (struct :`Yaw` 270.0) _lerp_3 true) false false)
                          (`SceneComponent.K2_SetRelativeRotation` _dog_head_1 (`KismetMathLibrary.RLerp` (`SceneComponent.RelativeRotation` _dog_head_1) (struct :`Yaw` 90.0) _lerp_3 true) false false))
                        (:`Finished`
                          (set `self.CanTurn?` false)))))
                  (else
                    (goto _label :!via `PlayFromStart`)))))))
        (else
          (for _array_element_2 (`self.CollisionBoxes`)
            (for _array_element_3 (`self.RequiredPuzzlePieces`)
              (if (not (`KismetArrayLibrary.Array_Contains` (`PrimitiveComponent.GetOverlappingComponents` _array_element_2) _array_element_3))
                (set `self.ContainsAllPieces` false)))
            (if (`self.ContainsAllPieces`)
              (set `self.BoxContainsPieces` _array_element_2)
              (set `self.puzzle1Solved` true)
              (break)
              (else
                (set `self.ContainsAllPieces` true)))))))))

(event `self.ReceiveBeginPlay`
  ;[1 1 1] setup
  (set `self.RubiksCube` (`|MakeArray` (`self.0_0_1`) (`self.0_1_1`) (`self.0_1_0`) (`self.1_0_0`) (`self.0_0_0`) (`self.1_0_1`) (`self.1_1_1`) (`self.1_1_0`) :!type "PrimitiveComponent Object Reference"))
  (`self.EnableInput` (`GameplayStatics.GetPlayerController` 0))
  (set `self.RequiredPuzzlePieces` (`|MakeArray` (`self.dog head 3`) (`self.dog head 2`) (`self.dog head 1`) (`self.stub`) :!type "PrimitiveComponent Object Reference"))
  (set `self.CollisionBoxes` (`|MakeArray` (`self.Verticle Box Front`) (`self.Depth Box Front`) (`self.Depth Box Back`) (`self.Horizontal Box Back`) (`self.Horizontal Box Front`) (`self.Verticle Box Back`)))
  (bind _returnvalue (`MaterialInterface.GetBaseMaterial` (`PrimitiveComponent.GetMaterial` (`self.0_0_0`) 0)))
  (set `self.BaseMaterial` _returnvalue))

(event `self.ReceiveActorOnClicked`
  (params (ButtonPressed :type "Key Structure"))
  (bind (_bblockinghit _binitialoverlap _time _distance _location _impactpoint _normal _impactnormal _physmat _hitactor _hitcomponent) (`GameplayStatics.BreakHitResult` (`PlayerController.GetHitResultUnderCursorByChannel` (`GameplayStatics.GetPlayerController` 0) "TraceTypeQuery1" true)))
  ;[1 1 1] cube selection
  (if (and (`ActorComponent.ComponentHasTag` _hitcomponent "CollisionBox") (`self.CanTurn?`))
    (set `self.Out Overlapping Components` (`PrimitiveComponent.GetOverlappingComponents` _hitcomponent))
    (bind _overlapping_blocks (`self.GetOverlappingBlocks` (`self.Out Overlapping Components`)))
    (set `self.Overlapping Blocks` _overlapping_blocks)
    (set `self.SelectedCollisionBox` _hitcomponent)))

(event `InputAction|RotateLeft`
  (params (Key :type "Key Structure"))
  (bind _selectedcollisionbox (`self.SelectedCollisionBox`))
  (bind _roll (.roll (`self.Cube Current Relative Rotation`)))
  (bind _output (`|GetArrayItem` (`SceneComponent.GetParentComponents` _selectedcollisionbox)))
  ;[1 1 1] Turn surfaces
  (:`Pressed`
    (if (`self.CanTurn?`)
      (set `self.Direction` -1.0)
      (if (!= _selectedcollisionbox null)
        (set `self.Cube Current Relative Rotation` (`SceneComponent.RelativeRotation` _output) :!label _label_2)
        (for _array_element (`self.RubiksCube`)
          (`SceneComponent.K2_AttachToComponent` _array_element (`self.DefaultSceneRoot`) "None" "KeepWorld" "KeepWorld" "KeepWorld" true))
        (for _array_element_2 (`self.Overlapping Blocks`)
          (`SceneComponent.K2_AttachToComponent` _array_element_2 _output "None" "KeepWorld" "KeepWorld" "KeepWorld" true)
          (bind (_direction _lerp) (`Timeline|Turn` :!via `PlayFromStart`)
            (:`Update`
              (set `self.CanTurn?` false)
              (`SceneComponent.K2_SetRelativeRotation` _output (`KismetMathLibrary.MakeRotator` (`KismetMathLibrary.Lerp` _roll (+ _roll (* (`self.Direction`) 90.0)) _lerp) (.pitch (`self.Cube Current Relative Rotation`)) (.yaw (`self.Cube Current Relative Rotation`))) false false))
            (:`Finished`
              (set `self.CanTurn?` true))))))))

(event `InputAction|RotateRight`
  (params (Key :type "Key Structure"))
  ;[1 1 1] Turn surfaces
  (:`Pressed`
    (if (`self.CanTurn?`)
      (set `self.Direction` 1.0)
      (if (!= (`self.SelectedCollisionBox`) null)
        (goto _label_2)))))

(event `self.dog head 1.OnClicked`
  (params (TouchedComponent :type "PrimitiveComponent Object Reference") (ButtonPressed :type "Key Structure"))
  ;[1 1 1] dogs rotations
  (if (`self.CanTurn?`)
    (set `self.DogCurrentRelativeRotation` (`SceneComponent.RelativeRotation` TouchedComponent))
    (bind (_direction _lerp) (`Timeline|dog turn 1` :!via `PlayFromStart`)
      (:`Update`
        (set `self.CanTurn?` false)
        (`self.Dog Lerp Rotate` TouchedComponent _lerp))
      (:`Finished`
        (set `self.CanTurn?` true)))))

(event `self.dog head 2.OnClicked`
  (params (TouchedComponent :type "PrimitiveComponent Object Reference") (ButtonPressed :type "Key Structure"))
  ;[1 1 1] dogs rotations
  (if (`self.CanTurn?`)
    (set `self.DogCurrentRelativeRotation` (`SceneComponent.RelativeRotation` TouchedComponent))
    (bind (_direction _lerp) (`Timeline|dog turn 2` :!via `PlayFromStart`)
      (:`Update`
        (set `self.CanTurn?` false)
        (`self.Dog Lerp Rotate` TouchedComponent _lerp))
      (:`Finished`
        (set `self.CanTurn?` true)))))

(event `InputAction|RotateUp`
  (params (Key :type "Key Structure"))
  (bind _roll (.roll (`self.RubiksCubeCurrentRotation`)))
  ;[1 1 1] whole cube rotation
  (:`Pressed`
    (if (`self.CanTurn?`)
      (if (== (`self.SelectedCollisionBox`) null)
        (set `self.Direction` 1.0 :!label _label_3)
        (set `self.RubiksCubeCurrentRotation` (`self.K2_GetActorRotation`))
        (bind (_direction _lerp) (`Timeline|rubiks cube rotation up and down` :!via `PlayFromStart`)
          (:`Update`
            (set `self.CanTurn?` false)
            (`self.K2_SetActorRotation` (`KismetMathLibrary.MakeRotator` (`KismetMathLibrary.Lerp` _roll (+ _roll (* (`self.Direction`) 180.0)) _lerp) (.pitch (`self.RubiksCubeCurrentRotation`)) (.yaw (`self.RubiksCubeCurrentRotation`)))))
          (:`Finished`
            (set `self.CanTurn?` true)))))))

(event `Flip`
  ;[1 1 1] whole cube rotation
  (goto _label_3))

(event `self.dog head 3.OnClicked`
  (params (TouchedComponent :type "PrimitiveComponent Object Reference") (ButtonPressed :type "Key Structure"))
  ;[1 1 1] dogs rotations
  (if (`self.CanTurn?`)
    (set `self.DogCurrentRelativeRotation` (`SceneComponent.RelativeRotation` TouchedComponent))
    (bind (_direction _lerp) (`Timeline|dog turn 3` :!via `PlayFromStart`)
      (:`Update`
        (set `self.CanTurn?` false)
        (`self.Dog Lerp Rotate` TouchedComponent _lerp))
      (:`Finished`
        (set `self.CanTurn?` true)))))

(event `InputAxis|TurnX`
  (params (AxisValue :type "Float (single-precision)"))
  ;[1 1 1] whole cube rotation
  (if (and (`self.IsLMBDown`) (`self.CanTurn?`))
    (`self.K2_AddActorWorldRotation` (`KismetMathLibrary.MakeRotator` 0.0 0.0 (* AxisValue -3.0)))))

(event `InputAction|Drag`
  (params (Key :type "Key Structure"))
  ;[1 1 1] whole cube rotation
  (:`Pressed`
    (set `self.IsLMBDown` true))
  (:`Released`
    (set `self.IsLMBDown` false)))

(event `Key|P`
  (params (Key :type "Key Structure"))
  (bind _returnvalue (`GameplayStatics.GetPlayerController` 0))
  (:`Pressed`
    (`/Engine/EditorBlueprintResources/StandardMacros.FlipFlop`
      (:`A`
        (bind _returnvalue_2 (`|CreateWidget` "/Game/UI/RulesWidget.RulesWidget_C"))
        (`UserWidget.AddToViewport` _returnvalue_2 0)
        (`GameplayStatics.SetGamePaused` true)
        (set `PlayerController.bShowMouseCursor` true _returnvalue))
      (:`B`
        (`Widget.RemoveFromParent` _returnvalue_2)
        (`GameplayStatics.SetGamePaused` false)
        (set `PlayerController.bShowMouseCursor` false _returnvalue)))))

(event `Key|T`
  (params (Key :type "Key Structure"))
  (:`Pressed`
    (bind _returnvalue (`|CreateWidget` "/Game/UI/WordingForPuzzleone.WordingForPuzzleone_C"))
    (`UserWidget.AddToViewport` _returnvalue 0)))

(fn `Dog Lerp Rotate`
  (params (TargetComponent :type "SceneComponent Object Reference") (Lerp :type "Float (double-precision)"))
  (bind _yaw (.yaw (`self.DogCurrentRelativeRotation`)))
  (`SceneComponent.K2_SetRelativeRotation` TargetComponent (`KismetMathLibrary.MakeRotator` (.roll (`self.DogCurrentRelativeRotation`)) (.pitch (`self.DogCurrentRelativeRotation`)) (`KismetMathLibrary.Lerp` _yaw (+ _yaw 90.0) Lerp)) false false))

(fn `GetOverlappingBlocks`
  (params (OverlappingComponents :type "Array of PrimitiveComponent Object Reference"))
  (returns (`Overlapping Blocks` :type "Array of PrimitiveComponent Object Reference"))
  (locals (Blocks :type "Array of PrimitiveComponent Object Reference"))
  (`KismetArrayLibrary.Array_Clear` (`self.Overlapping Blocks`))
  (`KismetArrayLibrary.Array_Clear` (`local.Blocks`))
  (for _array_element OverlappingComponents
    (if (`ActorComponent.ComponentHasTag` _array_element "CubeBlock")
      (`KismetArrayLibrary.Array_Add` (`local.Blocks`) _array_element)
      (`PrimitiveComponent.SetMaterial` _array_element 0 "/Game/Geometry/Meshes/textures/Ebase_Emissive_Inst.Ebase_Emissive_Inst")))
  (return (`local.Blocks`)))

(fn `HighlightCube`
  (params (Color :type "LinearColor Structure"))
  (returns (SelectedCube :type "PrimitiveComponent Object Reference"))
  (bind (_bblockinghit _binitialoverlap _time _distance _location _impactpoint _normal _impactnormal _physmat _hitactor _hitcomponent) (`GameplayStatics.BreakHitResult` (`PlayerController.GetHitResultUnderCursorByChannel` (`GameplayStatics.GetPlayerController` 0) "TraceTypeQuery1" true)))
  (bind _returnvalue (`PrimitiveComponent.CreateDynamicMaterialInstance` _hitcomponent 0 (`PrimitiveComponent.GetMaterial` _hitcomponent 0) "None"))
  (`MaterialInstanceDynamic.SetVectorParameterValue` _returnvalue "Emissive" Color)
  (`PrimitiveComponent.SetMaterial` _hitcomponent 0 _returnvalue)
  (return null))

(fn `Randomize`
  (locals (TempTransform :type "Array of Transform Structure") (ChildTempTransform :type "Transform Structure"))
  (for (_array_element _array_index) (`self.RubiksCube`)
    (`KismetArrayLibrary.Array_Set` (`local.TempTransform`) _array_index (`SceneComponent.GetRelativeTransform` _array_element)))
  (`KismetArrayLibrary.Array_Shuffle` (`local.TempTransform`))
  (for (_array_element_2 _array_index_2) (`self.RubiksCube`)
    (bind _returnvalue (`SceneComponent.GetChildComponent` _array_element_2 0))
    (`/Engine/EditorBlueprintResources/StandardMacros.IsValid` _returnvalue
      (:`Is Valid`
        (set `local.ChildTempTransform` (`SceneComponent.GetRelativeTransform` _returnvalue))
        (bind _output (`|GetArrayItem` (`local.TempTransform`) _array_index_2))
        (`SceneComponent.K2_SetRelativeTransform` _array_element_2 _output false false)
        (`SceneComponent.K2_SetRelativeTransform` _returnvalue (`local.ChildTempTransform`) false false))
      (:`Is Not Valid`
        (`SceneComponent.K2_SetRelativeTransform` _array_element_2 _output false false)))))

(fn `RotateAround`
  (params (Center :type "Vector Structure") (Rotation :type "Rotator Structure") (Distance :type "Float (double-precision)"))
  (returns (OutPoint :type "Vector Structure"))
  (return (+ Center (* (`KismetMathLibrary.GetForwardVector` Rotation) Distance))))

(fn `UnHighlightCube`
  (params (Color :type "LinearColor Structure") (Target :type "PrimitiveComponent Object Reference"))
  (`PrimitiveComponent.SetMaterial` Target 0 (`self.BaseMaterial`)))

(fn `UserConstructionScript`)